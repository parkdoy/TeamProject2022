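; Player building component that places, rotates, cycles and removes structures defined in a buildable data table.
; A timer-looped BuildCycle traces from the camera to move a ghost mesh, snapping it to collision boxes that hit actors report through a message.
; A box overlap check tints the ghost green or red and decides whether placement is allowed.
; Placed actors receive a completion message and are tracked, so only those can be removed.
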(event Custom|BuildDelay
  (if (Variables|기본/디폴트|GetIsbuildModeOn)
    (Utilities|Time|SetTimerbyFunctionName 0 "BuildCycle" 0.01)
    (else
      (Variables|기본/디폴트|SetIsbuildModeOn false)
      (Variables|Default|SetCanBuild false)
      (Utilities|IsValid (Variables|컴포넌트|GetBuildGhost)
        (:Is%20Valid
          ;[1 1 1] 코멘트
          (Default|DestroyComponent (Variables|Default|GetPlayerRef) (Variables|컴포넌트|GetBuildGhost)))))))

(event Custom|LaunchBuildMode
  ;[1 1 1] 코멘트
  (if (Variables|기본/디폴트|GetIsbuildModeOn)
    (CallFunction|StopBuildMode)
    (else
      (Variables|기본/디폴트|SetIsbuildModeOn true)
      (CallFunction|BuildCycle))))

(event Custom|StopBuildMode
  (Variables|기본/디폴트|SetIsbuildModeOn false)
  (Variables|Default|SetCanBuild false)
  (Utilities|IsValid (Variables|컴포넌트|GetBuildGhost)
    (:Is%20Valid
      ;[1 1 1] 코멘트
      (Default|DestroyComponent (Variables|Default|GetPlayerRef) (Variables|컴포넌트|GetBuildGhost)))))

(event EventBeginPlay
  (bind _outrownames (DataTable|GetDataTableRowNames "/Game/BluePrints/Building/BuildableDataTable.BuildableDataTable"))
  (for _array_element _outrownames
    (bind _returnvalue (Utilities|GetDataTableRow "/Game/BluePrints/Building/BuildableDataTable.BuildableDataTable" _array_element)
      (:then
        (Utilities|Array|Add (Variables|Default|GetBuildables) _returnvalue)))))

(fn SpawnBuildGhost
  (bind _returnvalue (Game|AddComponentbyClass (Variables|Default|GetPlayerRef) "/Script/Engine.StaticMeshComponent" false (Variables|Default|GetBuildTransform)))
  (bind _output_get (Variables|컴포넌트|SetBuildGhost _returnvalue))
  (Components|StaticMesh|SetStaticMesh _output_get (.mesh (Utilities|Array|Get(acopy) (Variables|Default|GetBuildables) (Variables|Default|GetBuildID))))
  (Collision|SetCollisionEnabled (Variables|컴포넌트|GetBuildGhost) "NoCollision"))

(fn GiveBuildColor
  (params (IsGreen :type Boolean))
  (Variables|Default|SetCanBuild IsGreen)
  (for _index (range 0 (- (Rendering|Material|GetNumMaterials (Variables|컴포넌트|GetBuildGhost)) 1))
    (if IsGreen
      (Rendering|Material|SetMaterial (Variables|컴포넌트|GetBuildGhost) _index "/Game/BluePrints/Material/M_GreenColor.M_GreenColor")
      (else
        (Rendering|Material|SetMaterial (Variables|컴포넌트|GetBuildGhost) _index "/Game/BluePrints/Material/M_RedColor.M_RedColor"))))
  (Transformation|SetWorldTransform (Variables|컴포넌트|GetBuildGhost) (Variables|Default|GetBuildTransform) false false))

(fn BuildCycle
  (bind _camera (Variables|Component|GetCamera))
  (bind _returnvalue (Transformation|GetWorldLocation _camera))
  (bind _returnvalue_2 (Math|Vector|GetForwardVector _camera))
  (bind (_outhit _returnvalue_3) (Collision|LineTraceByChannel (+ _returnvalue (* _returnvalue_2 3.5e+02)) (+ _returnvalue (* _returnvalue_2 1e+03)) (.tracechannel (Utilities|Array|Get(acopy) (Variables|Default|GetBuildables) (Variables|Default|GetBuildID))) true 0 "None"))
  (if _returnvalue_3
    (Variables|Default|SetBuildTransform (Math|Transform|MakeTransform (.ImpactPoint (Collision|BreakHitResult _outhit)) (.rotation (Variables|Default|GetBuildTransform)) (.scale (Variables|Default|GetBuildTransform))))
    (Variables|Default|SetHit%20Actor (.HitActor (Collision|BreakHitResult _outhit)))
    (Variables|컴포넌트|SetHit%20Component (.HitComponent (Collision|BreakHitResult _outhit)))
    (Utilities|IsValid (Variables|컴포넌트|GetBuildGhost)
      (:Is%20Valid
        ;[1 1 1] 스냅
        (bind (_found _transform) (CallFunction|DetectBoxCollision))
        (if _found
          (Variables|Default|SetBuildTransform _transform))
        (bind _hit (CallFunction|CheckforOverlap))
        (if _hit
          (CallFunction|GiveBuildColor false)
          (else
            (CallFunction|GiveBuildColor true)))
        (CallFunction|BuildDelay))
      (:Is%20Not%20Valid
        (CallFunction|SpawnBuildGhost)
        (CallFunction|BuildDelay :!label _label)))
    (else
      (Variables|Default|SetBuildTransform (Math|Transform|MakeTransform (.TraceEnd (Collision|BreakHitResult _outhit)) (.rotation (Variables|Default|GetBuildTransform)) (.scale (Variables|Default|GetBuildTransform))))
      (Utilities|IsValid (Variables|컴포넌트|GetBuildGhost)
        (:Is%20Valid
          (CallFunction|GiveBuildColor false)
          (goto _label))
        (:Is%20Not%20Valid
          (CallFunction|SpawnBuildGhost)
          (goto _label))))))

(fn ChangeMesh
  (Components|StaticMesh|SetStaticMesh (Variables|컴포넌트|GetBuildGhost) (.mesh (Utilities|Array|Get(acopy) (Variables|Default|GetBuildables) (Variables|Default|GetBuildID)))))

(fn SpawnBuild
  (params (IsbuildModeOn :type Boolean) (CanBuild :type Boolean) (ID :type Integer) (ST_Data :type Array%20of%20S%20Build%20Database%20Structures) (Transform :type Transform) (Character :type Third%20Person%20Character%20Object%20Reference))
  (if (and IsbuildModeOn CanBuild)
    (bind _returnvalue (Game|SpawnActorfromClass (.actor (Utilities|Array|Get(acopy) ST_Data ID)) Transform "Undefined" (Components|GetOwner Character) 0))
    (Class|BuildInterface|CompleteBuild(Message) _returnvalue)
    (Utilities|Set|Add (Variables|Default|GetSaveBuild) _returnvalue)))

(fn DetectBoxCollision
  ;[1 1 1] 매쉬에 붙어 있는 콜리전 박스를 찾는다
  (bind _boxes (Class|BuildInterface|ReturnBoxesCollision(Message) (Variables|Default|GetHit%20Actor)))
  (bind _array_element (Utilities|Array|ForEachLoopwithBreak _boxes :!label _label)
    (:LoopBody
      (if (== _array_element (Variables|컴포넌트|GetHit%20Component))
        (LocalVariables|SetLocalFound true)
        (goto _label Break)))
    (:Completed
      (return (LocalVariables|GetLocalFound) (Transformation|GetWorldTransform (Variables|컴포넌트|GetHit%20Component))))))

(fn CheckforOverlap
  (bind _buildghost (Variables|컴포넌트|GetBuildGhost))
  (bind (_origin _boxextent) (Collision|GetComponentBounds _buildghost))
  (bind _returnvalue (/ _boxextent 1.3))
  (bind _returnvalue_2 (Collision|BoxTraceByChannel _origin _origin (Math|Vector|MakeVector (.x _returnvalue) (.y _returnvalue) 1e+01) "0, 0, 0" "TraceTypeQuery1" false 0 "ForOneFrame"))
  (return _returnvalue_2))

(fn Initialize
  (params (player :type Third%20Person%20Character%20Object%20Reference) (Camera :type Camera%20Component%20Object%20Reference))
  (Variables|Default|SetPlayerRef player)
  (Variables|Component|SetCamera Camera))

(fn ChangeGhostmesh
  (params (NewParam :type Boolean))
  (bind _buildables (Variables|Default|GetBuildables))
  (bind _returnvalue (Utilities|Array|Length _buildables))
  (if NewParam
    (Utilities|CheckBuildModeon
      (:True
        (Variables|Default|SetBuildID (Math|Integer|Clamp(Integer) (+ (Variables|Default|GetBuildID) 1) 0 (- _returnvalue 1)))))
    (else
      (Utilities|CheckBuildModeon
        (:True
          (Variables|Default|SetBuildID (Math|Integer|Clamp(Integer) (- (Variables|Default|GetBuildID) 1) 0 _returnvalue))))))
  (CallFunction|ChangeMesh))

(fn AddRotate
  ;[1 1 1] 로테이션
  (Utilities|CheckBuildModeon
    (:True
      (Variables|Default|SetBuildTransform (Math|Transform|MakeTransform (.location (Variables|Default|GetBuildTransform)) (Math|Rotator|CombineRotators (.rotation (Variables|Default|GetBuildTransform)) "0,5.000000, 0") (.scale (Variables|Default|GetBuildTransform))))
      (Utilities|Time|SetTimerbyFunctionName 0 "Add Rotate" 0.01))))

(fn ClearAddRotate
  (Utilities|Time|ClearTimerbyFunctionName 0 "Add Rotate"))

(fn AddRotateInverse
  ;[1 1 1] 로테이션
  (Utilities|CheckBuildModeon
    (:True
      (Variables|Default|SetBuildTransform (Math|Transform|MakeTransform (.location (Variables|Default|GetBuildTransform)) (Math|Rotator|CombineRotators (.rotation (Variables|Default|GetBuildTransform)) "0,-5.000000, 0") (.scale (Variables|Default|GetBuildTransform))))
      (Utilities|Time|SetTimerbyFunctionName 0 "AddRotateInverse" 0.01))))

(fn ClearAddRotateInverse
  (Utilities|Time|ClearTimerbyFunctionName 0 "AddRotateInverse"))

(fn RemoveBuild
  (bind _camera (Variables|Component|GetCamera))
  (bind _returnvalue (Transformation|GetWorldLocation _camera))
  (bind _returnvalue_2 (Math|Vector|GetForwardVector _camera))
  (bind (_outhit _returnvalue_3) (Collision|LineTraceByChannel (+ _returnvalue (* _returnvalue_2 3.5e+02)) (+ _returnvalue (* _returnvalue_2 1e+03)) "TraceTypeQuery1" false 0 "ForDuration" true "(R=0.019954,G=0.033308,B=1.000000,A=1.000000)"))
  (if _returnvalue_3
    (bind _output_get (LocalVariables|SetLocalHitActor (.HitActor (Collision|BreakHitResult _outhit))))
    (if (Utilities|Set|Contains (Variables|Default|GetSaveBuild) _output_get)
      (Actor|DestroyActor _output_get))))

(fn Trace
  (bind _camera (Variables|Component|GetCamera))
  (bind _returnvalue (Transformation|GetWorldLocation _camera))
  (bind _returnvalue_2 (Math|Vector|GetForwardVector _camera))
  (bind (_outhit _returnvalue_3) (Collision|LineTraceByChannel (+ _returnvalue (* _returnvalue_2 3.5e+02)) (+ _returnvalue (* _returnvalue_2 1e+03)) "TraceTypeQuery1" false 0 "ForDuration"))
  (if _returnvalue_3
    (bind _output_get (Variables|Default|SetHit%20Actor (.HitActor (Collision|BreakHitResult _outhit))))
    (return _output_get)))